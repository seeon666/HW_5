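; Flashing light actor that blinks a PointLight indefinitely from BeginPlay, after applying LightColor.
; A loop of FlashCount iterations fires a FlipFlop that switches the light's visibility, then calls a Delay of FlashSpeed that re-enters the loop.
; Because the Delay does not pause the loop, each pass's toggles run in one frame, so only an odd FlashCount visibly alternates the light.
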(event Collision|EventActorBeginOverlap
  (params (OtherActor :type Actor%20Object%20Reference)))

(event EventTick
  (params (DeltaSeconds :type Float%20%28single-precision%29)))

(event EventBeginPlay
  (Rendering|Components|Light|SetLightColor (Variables|Default|GetPointLight) (Variables|Default|GetLightColor) true)
  (for _index (range 1 (Variables|Default|GetFlashCount)) :!label _label
    (Utilities|FlowControl|FlipFlop
      (:A
        (Rendering|SetVisibility (Variables|Default|GetPointLight) true false))
      (:B
        (Rendering|SetVisibility (Variables|Default|GetPointLight) false false)))
    (Utilities|FlowControl|Delay (Variables|Default|GetFlashSpeed))
    (goto _label)))

(fn ConstructionScript)